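; Trigger actor that activates the boss enemy when the player character walks into it.
; On BeginPlay it caches the first Bp_character and BP_Enemy_BOSS found in the level.
; When its Trigger component is overlapped by that character, it waits briefly, then sets the boss's ACTIVEwhenTrigger flag to true.
; It does not spawn the boss, despite the asset name.
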(event `self.ReceiveBeginPlay`
  (bind _returnvalue (`GameplayStatics.GetActorOfClass` "/Game/Blueprints/Character/bp_character.bp_character_C"))
  (set `self.Char` _returnvalue)
  (bind _returnvalue_2 (`GameplayStatics.GetActorOfClass` "/Game/Blueprints/Enemies/BP_Enemy_BOSS.BP_Enemy_BOSS_C"))
  (set `self.boss` _returnvalue_2))

(event `self.trigger.OnComponentBeginOverlap`
  (params (OverlappedComponent :type "PrimitiveComponent Object Reference") (OtherActor :type "Actor Object Reference") (OtherComp :type "PrimitiveComponent Object Reference") (OtherBodyIndex :type Integer) (bFromSweep :type Boolean) (SweepResult :type "HitResult Structure (by ref)"))
  (if (== OtherActor (`self.Char`))
    (`KismetSystemLibrary.Delay` 0.2)
    (set `/Game/Blueprints/Enemies/BP_Enemy_BOSS.ACTIVEwhenTrigger` true (`self.boss`))))

(fn `UserConstructionScript`)