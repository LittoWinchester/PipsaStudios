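; Trigger volume that handles the player falling, handing the character a destination to be teleported to.
; On BeginPlay it caches the character, and its box overlap reacts only to that character's walk collision.
; It reads the location of the WhereTPFall actor, waits briefly, plays a drop sound, then passes that location to the character's FNFallingMessage.
; A debug print remains live, while a stage-name teleport lookup is left disconnected.
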(event `self.ReceiveBeginPlay`
  (`parent.ReceiveBeginPlay`)
  (set `self.char` (`self.CHARACTER_REF`)))

(event `self.Box.OnComponentBeginOverlap`
  (params (OverlappedComponent :type "PrimitiveComponent Object Reference") (OtherActor :type "Actor Object Reference") (OtherComp :type "PrimitiveComponent Object Reference") (OtherBodyIndex :type Integer) (bFromSweep :type Boolean) (SweepResult :type "HitResult Structure (by ref)"))
  (if (== OtherComp (`/Game/Blueprints/Character/bp_character.WalkCollision` (`self.char`)))
    (bind _location (`self.Set Place`))
    (`KismetSystemLibrary.PrintString` "TOCASTE")
    (`KismetSystemLibrary.Delay` 0.3)
    (`GameplayStatics.PlaySound2D` "/Game/Music_Sounds/drop.drop" 1.0 1.0 0.0 null null)
    (message `/Game/Blueprints/Triggers/BPI_TriggerRoof.FN_Falling` OtherActor _location)))

(fn `Set Place`
  (returns (location :type "Vector Structure"))
  (return (`self.K2_GetActorLocation` (`self.WhereTPFall`))))

(fn `UserConstructionScript`)