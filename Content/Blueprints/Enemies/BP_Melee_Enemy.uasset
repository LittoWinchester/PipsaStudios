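; Melee enemy that chases Bp_character and deals damage in close range, with room-based activation through EnemyStartFollow.
; A looping timer drives Following, which moves and yaws the enemy or attacks with delays, using capsule overlaps and distance checks.
; Damage, melee hits and charm touches reduce parent-managed health; death destroys it, granting a door key if flagged ENEMYCLAVE.
; Movement normalizes the player's position rather than the direction toward them; CheckDirection only prints debug text.
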(event `Hit visual representation`
  (bind _sprite (`self.Sprite`))
  (bind _sprite_2 (`self.Sprite`))
  (`/Engine/EditorBlueprintResources/StandardMacros.IsValid` _sprite_2
    (:`Is Valid`
      (`PaperFlipbookComponent.SetSpriteColor` _sprite_2 (struct :`R` 1.0 :`B` 0.084659 :`A` 1.0))
      (`KismetSystemLibrary.Delay` 0.2)
      (`/Engine/EditorBlueprintResources/StandardMacros.IsValid` _sprite
        (:`Is Valid`
          (`PaperFlipbookComponent.SetSpriteColor` _sprite (struct :`R` 1.0 :`G` 1.0 :`B` 1.0 :`A` 1.0)))))))

(event `EnemyStartFollow`
  (params (`Action Value` :type Boolean) (Room :type Integer) (Activate :type "Array of /Game/Blueprints/Enemies/BP_Melee_Enemy Object Reference"))
  ;[0.3291 1 0.7119] FN_CHECK ROOM ENEMYS
  (for _array_element Activate
    (if (`KismetSystemLibrary.IsValid` _array_element)
      (`self.FN_StartChase` _array_element) ; ERROR IF ONE OF THE ARRAY DIES BEFORE START
    )))

(event `FN_StartChase`
  ;[1 0.2636 0.03237] MOVEMENT ENEMYS
  (`KismetSystemLibrary.K2_SetTimerDelegate` (delegate `Following`) 0.1 true)
  (bind _returnvalue (`GameplayStatics.GetActorOfClass` "/Game/Blueprints/Character/bp_character.bp_character_C"))
  (set `self.Objective` _returnvalue))

(event `Following`
  ;[1 0.2636 0.03237] MOVEMENT ENEMYS
  (if (and (stale `EnemyStartFollow` `Action Value`) (not (`self.touching`)))
    (`self.FNchase`)
    (`self.CheckDirection`)
    (elif (`self.touching`)
      (if (`self.DoneDamage`)
        (`KismetSystemLibrary.Delay` 1.5))
      (message `/Game/Blueprints/BPI_Damage.BPI_Damage` (`self.Objective`) true (`self.Damage`))
      (set `self.ATACO` false)
      (set `self.DoneDamage` true)
      (`KismetSystemLibrary.Delay` 1.1)
      (bind _melee_ (`self.FNCheckDistance`))
      (bind _output_get (set `self.touching` _melee_))
      (`KismetSystemLibrary.PrintString` (`KismetStringLibrary.Conv_BoolToString` _output_get) true true (struct :`G` 0.01475 :`B` 1.0 :`A` 1.0))
      (else
        (`self.FNchase`)
        (`self.CheckDirection`)))))

(event `self.ReceiveBeginPlay`
  (`parent.ReceiveBeginPlay`))

(event `self.ReceiveTick`
  (params (DeltaSeconds :type "Float (single-precision)")))

(event `self.ReceiveAnyDamage`
  (params (Damage :type "Float (single-precision)") (DamageType :type "DamageType Object Reference") (InstigatedBy :type "Controller Object Reference") (DamageCauser :type "Actor Object Reference"))
  (`self.FN Reduce HP_PC` Damage)
  (`self.Hit visual representation`)
  (`KismetSystemLibrary.PrintString` (`KismetStringLibrary.Concat_StrStr` "ME QUITO " (`KismetStringLibrary.Conv_DoubleToString` Damage) "  MI VIDA ES" (`KismetStringLibrary.Conv_DoubleToString` (`self.PC_Health`))) true true (struct :`G` 0.089374 :`B` 1.0 :`A` 1.0)))

(event `self.CapsuleComponent.OnComponentBeginOverlap`
  (params (OverlappedComponent :type "PrimitiveComponent Object Reference") (OtherActor :type "Actor Object Reference") (OtherComp :type "PrimitiveComponent Object Reference") (OtherBodyIndex :type Integer) (bFromSweep :type Boolean) (SweepResult :type "HitResult Structure (by ref)"))
  (if (== OtherActor (`self.Objective`))
    (set `self.touching` true)))

(event `self.CapsuleComponent.OnComponentEndOverlap`
  (params (OverlappedComponent :type "PrimitiveComponent Object Reference") (OtherActor :type "Actor Object Reference") (OtherComp :type "PrimitiveComponent Object Reference") (OtherBodyIndex :type Integer))
  (if (== (`self.Objective`) OtherActor)
    (set `self.touching` false)))

(fn `BPI_PlayerMelee`
  (params (Hit :type Boolean) (DMG :type "Float (double-precision)"))
  (`self.FN Reduce HP_PC` DMG))

(fn `CheckDirection`
  (bind (_returnvalue_x _returnvalue_y) (`KismetMathLibrary.BreakVector` (`self.K2_GetActorLocation`)))
  (bind (_returnvalue_x_2 _returnvalue_y_2) (`KismetMathLibrary.BreakVector` (`self.K2_GetActorLocation` (`self.Objective`))))
  (`/Engine/EditorBlueprintResources/StandardMacros.IsValid` (`self.Sprite`)
    (:`Is Valid`
      (if (< _returnvalue_x _returnvalue_x_2)
        (set `self.GoingUp` true)
        (else
          (set `self.GoingUp` false)))
      (if (< _returnvalue_y _returnvalue_y_2)
        (set `self.GoingLeft` true)
        (else
          (set `self.GoingLeft` false)))
      (if (`self.GoingLeft`)
        (if (`self.GoingUp`)
          (`KismetSystemLibrary.PrintString` "Derecha")
          (else
            (`KismetSystemLibrary.PrintString` "IZQUIERDA")))
        (else
          (if (`self.GoingUp`)
            _
            (else
              _))
          (`KismetSystemLibrary.PrintString` "ARRIBA ?"))))))

(fn `FN Reduce HP_PC`
  (params (`DMG recive` :type "Float (double-precision)"))
  (bind _healt_actual (`parent.FN Reduce HP_PC` `DMG recive`))
  (if (<= _healt_actual 0.0)
    (if (`self.ENEMY CLAVE`)
      (`/Game/Blueprints/Character/bp_character.Get Key Door Enemys` (`self.Objective`) 0))
    (`self.K2_DestroyActor`)))

(fn `FN_Charm-enemy`
  (params (Touched :type Boolean))
  (returns (`Event Ghost` :type Boolean))
  (set `/Game/Blueprints/Character/bp_character.CharmKill?` true (`self.Objective`))
  (`KismetSystemLibrary.PrintString` (`KismetStringLibrary.Concat_StrStr` "TOQUE EL AMULETO " "AHHH ME MUERO ") true true (struct :`A` 1.0) 4.0)
  (`GameplayStatics.ApplyDamage` self 25.0)
  (return true))

(fn `FNchase`
  (bind (_returnvalue_roll _returnvalue_pitch) (`KismetMathLibrary.BreakRotator` (`self.K2_GetActorRotation`)))
  (bind (_returnvalue_roll_2 _returnvalue_pitch_2 _returnvalue_yaw) (`KismetMathLibrary.BreakRotator` (`KismetMathLibrary.FindLookAtRotation` (`self.K2_GetActorLocation`) (`self.K2_GetActorLocation` (`self.Objective`)))))
  (if (not (`self.touching`))
    (`self.K2_AddActorLocalOffset` (* (`KismetMathLibrary.Normal` (`self.K2_GetActorLocation` (`self.Objective`))) (`self.Speed`)))
    (bind _melee_ (`self.FNCheckDistance`))
    (`self.K2_SetActorRotation` (`KismetMathLibrary.MakeRotator` _returnvalue_roll _returnvalue_pitch _returnvalue_yaw))
    (`KismetSystemLibrary.PrintString` (`KismetStringLibrary.Conv_DoubleToString` (`KismetMathLibrary.Vector_Distance` (`self.K2_GetActorLocation`) (`self.K2_GetActorLocation` (`self.Objective`)))))
    (if _melee_
      (set `self.touching` true))))

(fn `FNCheckDistance`
  (returns (`Melee?` :type Boolean))
  (if (`self.touching`)
    (if (>= (`KismetMathLibrary.Vector_Distance` (`self.K2_GetActorLocation` (`self.Objective`)) (`self.K2_GetActorLocation`)) 170.0)
      (return false)
      (else
        (return true)))
    (elif (<= (`KismetMathLibrary.Vector_Distance` (`self.K2_GetActorLocation` (`self.Objective`)) (`self.K2_GetActorLocation`)) 170.0)
      (return true)
      (else
        (return false)))))

(fn `UserConstructionScript`)