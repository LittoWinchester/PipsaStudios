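; Enemy projectile that damages the player character on overlap and destroys itself, or expires two seconds after spawning.
; BeginPlay caches the Bp_character reference and picks a random sprite for the projectile.
; Each Tick steps it by Speed in local space along the normalized vector toward the point in VectorDirection, without delta-time scaling.
; Damage goes through an interface message; a Rotation helper orients the Box by direction quadrant but is not called here.
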(event `self.ReceiveBeginPlay`
  (bind _returnvalue (`GameplayStatics.GetActorOfClass` "/Game/Blueprints/Character/bp_character.bp_character_C"))
  (set `self.characterBP` _returnvalue)
  (`PaperSpriteComponent.SetSprite` (`self.AssetsArray`) (`|GetArrayItem` (`self.GetNewAsset`) (`KismetMathLibrary.RandomIntegerInRange` 0 4)))
  (`KismetSystemLibrary.Delay` 2.0)
  (`self.K2_DestroyActor`))

(event `self.ReceiveTick`
  (params (DeltaSeconds :type "Float (single-precision)"))
  (`self.Direction Proyectile` (`self.VectorDirection`)))

(event `self.Box.OnComponentBeginOverlap`
  (params (OverlappedComponent :type "PrimitiveComponent Object Reference") (OtherActor :type "Actor Object Reference") (OtherComp :type "PrimitiveComponent Object Reference") (OtherBodyIndex :type Integer) (bFromSweep :type Boolean) (SweepResult :type "HitResult Structure (by ref)"))
  (if (== (`self.characterBP`) OtherActor)
    (message `/Game/Blueprints/BPI_Damage.BPI_Damage` OtherActor false (`self.damgae`))
    (`self.K2_DestroyActor`)))

(fn `Direction Proyectile`
  (params (Vector :type "Vector Structure"))
  (set `self.VectorDirection` Vector)
  (`self.K2_AddActorLocalOffset` (* (`KismetMathLibrary.Normal` (- (`self.VectorDirection`) (`self.K2_GetActorLocation`))) (`self.speed`))))

(fn `getterActorForward`)

(fn `Rotation?`
  (params (Direction :type "Vector Structure"))
  (bind _returnvalue (> Direction_Y 0.0))
  (if (> Direction_X 0.0)
    (if _returnvalue
      (`KismetSystemLibrary.PrintString` "SALE PARA  DOWN")
      (`SceneComponent.K2_AddLocalRotation` (`self.Box`) (struct :`Pitch` 180.0 :`Yaw` 90.0) false false)
      (else
        (`KismetSystemLibrary.PrintString` "SALE PARA DERECHA ")
        (`SceneComponent.K2_AddLocalRotation` (`self.Box`) (struct :`Pitch` 180.0) false false)))
    (elif _returnvalue
      (`KismetSystemLibrary.PrintString` "SALE PARA  IZQ")
      (`SceneComponent.K2_AddLocalRotation` :`self` (`self.Box`))
      (else
        (`KismetSystemLibrary.PrintString` "SALE PARA UP ")
        (`SceneComponent.K2_AddLocalRotation` (`self.Box`) (struct :`Pitch` 180.0 :`Yaw` -90.0) false false)))))

(fn `UserConstructionScript`)