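; Two-phase boss enemy that, once trigger-activated and sighting the player, shows a boss health bar and starts chasing.
; Phase one uses a looping timer to slide its Box toward the player and deal contact damage on overlap.
; AnyDamage below half health turns it into a stationary poltergeist firing projectiles on sight; melee hits skip this check.
; Death hides the bar, drops a boss symbol key and destroys the actor.
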(event `TransformingOnPoltergeist`
  (bind _locationtransformonpoltergeist (`self.LocationTransformOnPoltergeist`))
  ;[0.1121 0.1281 1] TRANSFORM
  (`KismetSystemLibrary.Delay` 0.3)
  (`PaperSpriteComponent.SetSprite` (`self.PaperSprite`) "/Game/Art/Assets/Poltergeist/Poltergeist_CPT_Sprite.Poltergeist_CPT_Sprite")
  (`SceneComponent.SetVisibility` (`self.SpriteBoss`) false false)
  (`self.K2_SetActorLocation` _locationtransformonpoltergeist)
  (`SceneComponent.K2_SetRelativeLocation` (`self.CapsuleComponent`) _locationtransformonpoltergeist false false))

(event `EnemyStartFollow`
  (params (`Action Value` :type Boolean) (Room :type Integer) (Activate :type "Array of /Game/Blueprints/Enemies/BP_Melee_Enemy Object Reference"))
  ;[1 0 0.05706] NO VA
  ;;[0.3291 1 0.7119] FN_CHECK ROOM ENEMYS
)

(event `FN_StartChase`
  ;[0.8959 0.5907 1] MOVEMENT ENEMYS
  (bind _returnvalue (`KismetSystemLibrary.K2_SetTimerDelegate` (delegate `Following`) 0.1 true))
  (set `self.DeleteEventTimer` _returnvalue))

(event `Following`
  ;[0.8959 0.5907 1] MOVEMENT ENEMYS
  (if (and (`self.ONSeePawn`) (not (`self.touching`)))
    (`self.FNchase`)
    (`self.CheckDirection`)
    (elif (`self.touching`)
      (if (`self.ATACO`)
        (`KismetSystemLibrary.Delay` 0.8))
      (message `/Game/Blueprints/BPI_Damage.BPI_Damage` (`self.Objective`) true (`self.Damage`))
      (set `self.ATACO` true)
      (`KismetSystemLibrary.Delay` 0.8)
      (bind _melee_ (`self.FNCheckDistance`))
      (if _melee_
        (set `self.ATACO` true)
        (else
          (set `self.ATACO` false)))
      (set `self.touching` _melee_)
      (else
        (`self.FNchase`)
        (`self.CheckDirection`)))))

(event `self.ReceiveBeginPlay`
  (`parent.ReceiveBeginPlay`)
  (bind _returnvalue (`GameplayStatics.GetActorOfClass` "/Game/Blueprints/Character/bp_character.bp_character_C"))
  (set `self.Objective` _returnvalue)
  (set `self.ACTIVEwhenTrigger` false))

(event `self.ReceiveTick`
  (params (DeltaSeconds :type "Float (single-precision)")))

(event `self.PawnSensing.OnSeePawn`
  (params (Pawn :type "Pawn Object Reference"))
  (if (`self.ACTIVEwhenTrigger`)
    ;[0.1036 1 0.4193] ON SEE PAWN
    (set `self.PawnOnSee` Pawn)
    (if (not (`self.Instance2?`))
      (set `self.ONSeePawn` (== Pawn (`self.Objective`)))
      (if (not (`self.CHASE?`))
        (`self.FN_StartChase`)
        (set `self.CHASE?` true)
        (`self.CreateBarHP` true))
      (else
        (`self.SHOOT THINGS` Pawn)))))

(event `self.Box.OnComponentBeginOverlap`
  (params (OverlappedComponent :type "PrimitiveComponent Object Reference") (OtherActor :type "Actor Object Reference") (OtherComp :type "PrimitiveComponent Object Reference") (OtherBodyIndex :type Integer) (bFromSweep :type Boolean) (SweepResult :type "HitResult Structure (by ref)"))
  (if (== OtherComp (`/Game/Blueprints/Character/bp_character.Collision` (`self.Objective`)))
    (set `self.touching` true)))

(event `self.Box.OnComponentEndOverlap`
  (params (OverlappedComponent :type "PrimitiveComponent Object Reference") (OtherActor :type "Actor Object Reference") (OtherComp :type "PrimitiveComponent Object Reference") (OtherBodyIndex :type Integer))
  (if (== (`/Game/Blueprints/Character/bp_character.Collision` (`self.Objective`)) OtherComp)
    (set `self.touching` false)))

(event `self.ReceiveAnyDamage`
  (params (Damage :type "Float (single-precision)") (DamageType :type "DamageType Object Reference") (InstigatedBy :type "Controller Object Reference") (DamageCauser :type "Actor Object Reference"))
  (`self.FN Reduce HP_PC` Damage)
  (if (not (`self.Instance2?`))
    (`self.Instances` (`self.PC_Health`))))

(event `SHOOT THINGS`
  (params (Pawn :type "Pawn Object Reference"))
  ;[1 0.6583 0.1705] SHOOT
  (if (and (== Pawn (`self.Objective`)) (`self.CanShoot?`))
    (`KismetSystemLibrary.PrintString` "TE VEO LOQUITO " true true (struct :`R` 0.737742 :`G` 1.0 :`A` 1.0) 5.0)
    (`|SpawnActorFromClass` "/Game/Blueprints/Enemies/bp_Proyectil_Enemy.bp_Proyectil_Enemy_C" (`KismetMathLibrary.Conv_VectorToTransform` (`self.LocationTransformOnPoltergeist`)) "Undefined" "MultiplyWithRoot" null 15.0 0.0 (`self.K2_GetActorLocation` (`self.Objective`)) 10.0 null)
    (set `self.CanShoot?` false)
    (`KismetSystemLibrary.Delay` 1.0)
    (set `self.CanShoot?` true)))

(fn `ActiveTimer`)

(fn `BPI_PlayerMelee`
  (params (Hit :type Boolean) (DMG :type "Float (double-precision)"))
  (`self.FN Reduce HP_PC` DMG))

(fn `CheckDirection`
  (`/Engine/EditorBlueprintResources/StandardMacros.IsValid` (`self.SpriteBoss`)
    (:`Is Valid`
      (set `self.VectotBossRotation` (`KismetMathLibrary.Conv_RotatorToVector` (`KismetMathLibrary.FindLookAtRotation` (`SceneComponent.K2_GetComponentLocation` (`self.Box`)) (`self.K2_GetActorLocation` (`self.Objective`))))))))

(fn `CreateBarHP`
  (params (`ready?` :type Boolean))
  (bind _wbp_bosshpbar (`/Game/UI/UI_OverlayPrincipal.WBP_BOSSHPBAR` (`/Game/Blueprints/Character/bp_character.UI principal` (`self.Objective`))))
  (if `ready?`
    (set `Widget.Visibility` "Visible" _wbp_bosshpbar)
    (`/Game/UI/WBP_BOSSHPBAR.RefreshBossHpBar` _wbp_bosshpbar (`self.PC_Health_MAX`) (`self.PC_Health`))))

(fn `FN Reduce HP_PC`
  (params (`DMG recive` :type "Float (double-precision)"))
  (bind _objective (`self.Objective`))
  (bind _healt_actual (`parent.FN Reduce HP_PC` `DMG recive`))
  (`/Game/UI/WBP_BOSSHPBAR.RefreshBossHpBar` (`/Game/UI/UI_OverlayPrincipal.WBP_BOSSHPBAR` (`/Game/Blueprints/Character/bp_character.UI principal` (`self.Objective`))) (`self.PC_Health_MAX`) _healt_actual)
  (if (<= _healt_actual 0.0)
    (if (`self.ENEMY CLAVE`)
      (`/Game/Blueprints/Character/bp_character.Get Key Door Enemys` (`self.Objective`) 0))
    (`self.ActiveTimer`)
    (`|SpawnActorFromClass` "/Game/Blueprints/Objects/BP_SymbolKey.BP_SymbolKey_C" (`KismetMathLibrary.Conv_VectorToTransform` (`self.K2_GetActorLocation`)) "Undefined" "MultiplyWithRoot" null "BOSSKEY" "/Game/Art/Environment/Props/Amuleto2_128_Sprite.Amuleto2_128_Sprite" null)
    (set `Widget.Visibility` "Hidden" (`/Game/UI/UI_OverlayPrincipal.WBP_BOSSHPBAR` (`/Game/Blueprints/Character/bp_character.UI principal` _objective)))
    (`/Game/Blueprints/Character/bp_character.AddToKeyBag` _objective 0 "TIMERON")
    (`self.K2_DestroyActor`)))

(fn `FN_Charm-enemy`
  (params (Touched :type Boolean))
  (returns (`Event Ghost` :type Boolean))
  (set `/Game/Blueprints/Character/bp_character.CharmKill?` true (`self.Objective`))
  (`KismetSystemLibrary.PrintString` (`KismetStringLibrary.Concat_StrStr` "TOQUE EL AMULETO " "AHHH ME MUERO ") true true (struct :`A` 1.0) 4.0)
  (`GameplayStatics.ApplyDamage` self 25.0)
  (return true))

(fn `FNchase`
  (set `self.movementOK` true)
  (if (`self.touching`)
    _
    (elif (not (`self.Instance2?`))
      (`SceneComponent.K2_AddLocalOffset` (`self.Box`) (* (`KismetMathLibrary.Normal` (- (`self.K2_GetActorLocation` (`self.Objective`)) (`SceneComponent.K2_GetComponentLocation` (`self.Box`)))) (`self.Speed`)) false false)
      (bind _melee_ (`self.FNCheckDistance`))
      (if _melee_
        (set `self.touching` true)
        (set `self.movementOK` false)))))

(fn `FNCheckDistance`
  (returns (`Melee?` :type Boolean))
  (if (`self.touching`)
    (return true)
    (else
      (return false))))

(fn `GetterLocation`
  (set `self.Set Location Objec` (`self.K2_GetActorLocation` (`self.Objective`))))

(fn `Instances`
  (params (HP :type "Float (double-precision)"))
  (if (< HP (/ (`self.PC_Health_MAX`) 2.0))
    (set `self.Instance2?` true)
    (`KismetSystemLibrary.K2_ClearAndInvalidateTimerHandle` (`self.DeleteEventTimer`))
    (`self.TransformingOnPoltergeist`)
    (else
      (`KismetSystemLibrary.PrintString` (`KismetStringLibrary.Conv_DoubleToString` HP)))))

(fn `RotationBoss`
  (bind (_returnvalue_roll _returnvalue_pitch _returnvalue_yaw) (`KismetMathLibrary.BreakRotator` (`KismetMathLibrary.FindLookAtRotation` (`self.K2_GetActorLocation`) (`self.K2_GetActorLocation` (`self.Objective`)))))
  (`self.K2_SetActorRelativeRotation` (`KismetMathLibrary.MakeRotator` _returnvalue_roll _returnvalue_pitch _returnvalue_yaw)))

(fn `UserConstructionScript`)