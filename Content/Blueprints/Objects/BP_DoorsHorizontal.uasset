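; Horizontal 2D door that opens when the player's SymbolBag contains its KeyToOpen symbol.
; Overlapping Collision runs the key check, which either opens the door or calls FNDoorMessage on the overlapping actor to show a message, cleared on overlap end.
; Opening shifts the blocking Box away and swaps the closed Paper sprite for left and right open sprites.
; A close function exists but is never called here.
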(event `self.ReceiveBeginPlay`
  (`parent.ReceiveBeginPlay`)
  (set `self.Player` (`self.CHARACTER_REF`)))

(event `self.Collision.OnComponentBeginOverlap`
  (params (OverlappedComponent :type "PrimitiveComponent Object Reference") (OtherActor :type "Actor Object Reference") (OtherComp :type "PrimitiveComponent Object Reference") (OtherBodyIndex :type Integer) (bFromSweep :type Boolean) (SweepResult :type "HitResult Structure (by ref)"))
  (bind _closed_ (`self.checkOpenDoor` (`self.Is_Open`)))
  (if _closed_
    (message `/Game/Blueprints/Objects/BPI_PickMe.FN_Door` OtherActor true)
    (`KismetSystemLibrary.PrintString` "Hello")))

(event `self.Collision.OnComponentEndOverlap`
  (params (OverlappedComponent :type "PrimitiveComponent Object Reference") (OtherActor :type "Actor Object Reference") (OtherComp :type "PrimitiveComponent Object Reference") (OtherBodyIndex :type Integer))
  (message `/Game/Blueprints/Objects/BPI_PickMe.FN_Door` OtherActor false))

(fn `checkOpenDoor`
  (params (`IsOpen?` :type Boolean))
  (returns (`Closed?` :type Boolean))
  (if (not `IsOpen?`)
    (for _array_element (`/Game/Blueprints/Character/bp_character.SymbolBag` (`self.Player`))
      (if (== _array_element (`self.KeyToOpen`))
        (bind _is_open_now (`self.MoveDoorOpen`))
        (set `self.Is_Open` _is_open_now)
        (return false)))
    (return true)))

(fn `MoveDoorCLOSE`
  (returns (`IS OPEN NOW` :type Boolean))
  (`SceneComponent.K2_AddLocalOffset` (`self.Box`) (0.0 0.0 1000.0) false false)
  (`PaperSpriteComponent.SetSprite` (`self.PaperSpriteClose`) "/Game/Art/Environment/Props/T_PuertaH_2_Sprite.T_PuertaH_2_Sprite")
  (return false))

(fn `MoveDoorOpen`
  (returns (`IS OPEN NOW` :type Boolean))
  (`SceneComponent.K2_AddLocalOffset` (`self.Box`) (700.0 500.0 -1000.0) false false)
  (`SceneComponent.SetVisibility` (`self.PaperSpriteClose`) false false)
  (`SceneComponent.SetVisibility` (`self.PaperSpriteOpen_L`) true false)
  (`SceneComponent.SetVisibility` (`self.PaperSpriteOpen_R`) true false)
  (return true))

(fn `UserConstructionScript`)