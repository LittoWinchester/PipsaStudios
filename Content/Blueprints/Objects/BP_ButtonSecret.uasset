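; BP_ButtonSecret is a one-shot trigger that signals the library's secret door when its box is overlapped.
; On BeginPlay it finds BP_LibraryMovement; the first overlap calls its FNSecretDoorMessage, swaps the Paper sprite to a rune amulet and sets Actioned to block repeats.
; Disconnected nodes hold an unused E-key pickup that would add a key to the character's bag and destroy the actor.
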(event `self.ReceiveTick`
  (params (DeltaSeconds :type "Float (single-precision)")))

(event `self.ReceiveBeginPlay`
  (bind _returnvalue (`GameplayStatics.GetActorOfClass` "/Game/Blueprints/Objects/BP_LibraryMovement.BP_LibraryMovement_C"))
  (set `self.Library` _returnvalue))

(event `FN Button`
  ;[1 1 1] Add Items to bag
)

(event `self.BPI_GRAB`
  (params (`N Item` :type Integer))
  ;[1 1 1] Add Items to bag
)

(event `self.Box.OnComponentBeginOverlap`
  (params (OverlappedComponent :type "PrimitiveComponent Object Reference") (OtherActor :type "Actor Object Reference") (OtherComp :type "PrimitiveComponent Object Reference") (OtherBodyIndex :type Integer) (bFromSweep :type Boolean) (SweepResult :type "HitResult Structure (by ref)"))
  (if (not (`self.Actioned?`))
    (message `/Game/Blueprints/Objects/BPI_PickMe.FN_secretDoor` (`self.Library`) true)
    (`PaperSpriteComponent.SetSprite` (`self.PaperSprite`) "/Game/Art/Assets/ITEMS/Amuleto1_128_runa_Sprite.Amuleto1_128_runa_Sprite")
    (set `self.Actioned?` true)))

(event `self.Box.OnComponentEndOverlap`
  (params (OverlappedComponent :type "PrimitiveComponent Object Reference") (OtherActor :type "Actor Object Reference") (OtherComp :type "PrimitiveComponent Object Reference") (OtherBodyIndex :type Integer)))

(fn `FN_Charm-enemy`
  (params (Touched :type Boolean)))

(fn `getter e button`
  (returns (`E PRESS?` :type Boolean))
  (if (and (`/Game/Blueprints/Character/bp_character.E_button` (`self.Character`)) (`self.Overlapping`))
    (bind _output_get (set `self.Pressed E` true))
    (return _output_get)
    (else
      (bind _output_get_2 (set `self.Pressed E` false))
      (return _output_get_2))))

(fn `UserConstructionScript`)