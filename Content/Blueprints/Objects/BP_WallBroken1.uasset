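; BP_WallBroken1 is a damageable wall that moves when hit and is destroyed once its HP runs out.
; It extends a parent's HP logic, setting Broke when the reduced HP reaches zero or below.
; Damage runs the break check: a broken wall destroys itself, otherwise a timeline applies local offsets and re-runs the check on finish, looping until broken.
; Tick and the temblor function do nothing.
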(event `self.ReceiveBeginPlay`
  (`parent.ReceiveBeginPlay`))

(event `Move and destroy`
  (if (`self.Broke`) :!label _label
    (set `self.moving` false)
    (`self.K2_DestroyActor`)
    (else
      (set `self.moving` true)
      (bind (_direction _newtrack_0) (`Timeline|Timeline` :!via `PlayFromStart`)
        (:`Update`
          (`self.K2_AddActorLocalOffset` _newtrack_0))
        (:`Finished`
          (`self.Move and destroy`))))))

(event `self.ReceiveAnyDamage`
  (params (Damage :type "Float (single-precision)") (DamageType :type "DamageType Object Reference") (InstigatedBy :type "Controller Object Reference") (DamageCauser :type "Actor Object Reference"))
  (`self.FN Reduce HP_PC` Damage)
  (goto _label))

(event `self.ReceiveTick`
  (params (DeltaSeconds :type "Float (single-precision)"))
  (if (`self.moving`)
    _))

(fn `FN Reduce HP_PC`
  (params (`DMG recive` :type "Float (double-precision)"))
  (returns (`Healt actual` :type "Float (double-precision)"))
  (bind _healt_actual (`parent.FN Reduce HP_PC` `DMG recive`))
  (if (<= _healt_actual 0.0)
    (set `self.Broke` true)
    (return _healt_actual)))

(fn `HP_Start`
  (`parent.HP_Start`))

(fn `temblor`)

(fn `UserConstructionScript`)