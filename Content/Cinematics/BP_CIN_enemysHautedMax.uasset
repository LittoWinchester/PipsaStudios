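; Cinematic haunted-enemy actor with four ghost components that can split apart, disappear and reset.
; SPLITGHOST caches their world locations, instantly pushes each along its own local X or Z axis, then hides all four after a short delay.
; OriginalLocation restores the cached locations, prints a debug string and makes them visible again.
; Locations are cached on BeginPlay and again on every split, so splitting twice without a reset overwrites the origin.
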(event `self.ReceiveBeginPlay`
  (`self.orig_loc`))

(event `SPLITGHOST`
  (`self.orig_loc`)
  (`SceneComponent.K2_AddLocalOffset` (`self.G1`) (0.0 0.0 -200.0) false false)
  (`SceneComponent.K2_AddLocalOffset` (`self.G2`) (0.0 0.0 200.0) false false)
  (`SceneComponent.K2_AddLocalOffset` (`self.G3`) (150.0 0.0 0.0) false false)
  (`SceneComponent.K2_AddLocalOffset` (`self.G4`) (-150.0 0.0 0.0) false false)
  (`KismetSystemLibrary.Delay` 2.0)
  (`SceneComponent.SetVisibility` (`self.G4`) false false)
  (`SceneComponent.SetVisibility` (`self.G1`) false false)
  (`SceneComponent.SetVisibility` (`self.G3`) false false)
  (`SceneComponent.SetVisibility` (`self.G2`) false false))

(event `OriginalLocation`
  (`self.setlocationsOrigin`)
  (`SceneComponent.SetVisibility` (`self.G4`) true false)
  (`SceneComponent.SetVisibility` (`self.G1`) true false)
  (`SceneComponent.SetVisibility` (`self.G3`) true false)
  (`SceneComponent.SetVisibility` (`self.G2`) true false))

(fn `orig_loc`
  (set `self.G1L` (`SceneComponent.GetSocketLocation` (`self.G1`) "None"))
  (set `self.G2L` (`SceneComponent.GetSocketLocation` (`self.G2`) "None"))
  (set `self.G3L` (`SceneComponent.K2_GetComponentLocation` (`self.G3`)))
  (set `self.G4L` (`SceneComponent.K2_GetComponentLocation` (`self.G4`))))

(fn `setlocationsOrigin`
  (`SceneComponent.K2_SetWorldLocation` (`self.G1`) (`self.G1L`) false false)
  (`SceneComponent.K2_SetWorldLocation` (`self.G2`) (`self.G2L`) false false)
  (`SceneComponent.K2_SetWorldLocation` (`self.G3`) (`self.G3L`) false false)
  (`SceneComponent.K2_SetWorldLocation` (`self.G4`) (`self.G4L`) false false)
  (`KismetSystemLibrary.PrintString` "!!!!!!!!!!!!!!!!!!!!!!!!!!!!!!!!!!!!!!!!!!!"))

(fn `UserConstructionScript`)